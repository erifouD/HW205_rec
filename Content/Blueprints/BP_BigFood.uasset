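; BP_BigFood is a food actor, judging by its name, that announces itself with a sound and blinks while in the level.
; On BeginPlay it plays the S_Abitily sound in 2D, then enters an endless one-second Delay loop that toggles the visibility of fifteen plane components.
; It contains no overlap, tick or construction logic, so any effect of eating it is not defined in this graph.
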(event `self.ReceiveBeginPlay`
  (`GameplayStatics.PlaySound2D` "/Game/Sounds/S_Abitily.S_Abitily" 1.0 1.0 0.0 null null)
  (`KismetSystemLibrary.Delay` 1.0 :!label _label)
  (for _array_element (`|MakeArray` (`self.Plane1`) (`self.Plane2`) (`self.Plane3`) (`self.Plane4`) (`self.Plane5`) (`self.Plane6`) (`self.Plane7`) (`self.Plane8`) (`self.Plane9`) (`self.Plane10`) (`self.Plane11`) (`self.Plane12`) (`self.Plane13`) (`self.Plane14`) (`self.Plane15`))
    (`SceneComponent.ToggleVisibility` _array_element false))
  (goto _label))

(fn `UserConstructionScript`)