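; BP_Snake is the snake actor, handling game setup, score notification and the game-over screen.
; On BeginPlay it reads BPIns_Transfer from the game instance to set the starting element count and an inverted MovementSpeed, so higher speed settings give smaller values.
; AddScore calls ScoreAdded.
; EndPlay serves as the game-over trigger, creating WBP_GameEnded with the final score and showing the mouse cursor.
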(event `self.ReceiveEndPlay`
  (params (EndPlayReason :type "EEndPlayReason Enum" :default "Destroyed"))
  (bind _returnvalue (`GameplayStatics.GetPlayerController` 0))
  (bind _returnvalue_2 (`|CreateWidget` "/Game/Widgets/WBP_GameEnded.WBP_GameEnded_C"))
  (`UserWidget.AddToViewport` _returnvalue_2 0)
  (`TextBlock.SetText` (`/Game/Widgets/WBP_GameEnded.TextBlock_291` _returnvalue_2) (`KismetTextLibrary.Conv_StringToText` (`KismetStringLibrary.Concat_StrStr` (`self.TextScore`) (`KismetStringLibrary.Conv_IntToString` (`self.ScoreCount`)))))
  (if (`KismetSystemLibrary.IsValid` _returnvalue)
    (set `PlayerController.bShowMouseCursor` true _returnvalue)))

(event `self.ReceiveBeginPlay`
  (bind _asbpins_transfer (cast `/Game/Blueprints/BPIns_Transfer` (`GameplayStatics.GetGameInstance`)))
  (set `self.MovementSpeed` (/ (- 6.0 (`/Game/Blueprints/BPIns_Transfer.SpeedIns` _asbpins_transfer)) 10.0))
  (set `self.CountOfElementsOnStart` (`/Game/Blueprints/BPIns_Transfer.ElemsIns` _asbpins_transfer)))

(event `self.AddScore`
  (`self.ScoreAdded`))

(fn `UserConstructionScript`)